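; AI controller for guard NPCs that runs a behavior tree on patrol blackboard data and reacts to AI Perception updates.
; Sensed actors without the "Enemy" tag become the blackboard Enemy and focus target; losing the stimulus clears both, with debug prints along the way.
; Each tick, the controlled Ue4ASP_Character's Aiming and Shooting flags mirror whether a focus actor exists.
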(event OnTargetPerceptionUpdated(AIPerception)
  (params (Actor :type Actor%20Object%20Reference) (Stimulus :type AI%20Stimulus%20Structure))
  ;[1 1 1] Debug OnTargetPerceptionUpdated
  (if (not (Actor|ActorHasTag Actor "Enemy"))
    (if (.bSuccessfullySensed (Utilities|Struct|BreakAIStimulus Stimulus))
      (AI|Components|Blackboard|SetValueasObject (Variables|Default|GetBlackBoardComp) (Variables|Default|GetEnemy) Actor)
      (Development|PrintString "Enemy Set")
      (AI|SetFocus Actor)
      (CallFunction|PrintDebugString Stimulus Actor)
      (else
        (AI|Components|Blackboard|ClearValue (Variables|Default|GetBlackBoardComp) (Variables|Default|GetEnemy))
        (Development|PrintString "Enemy Cleared")
        (AI|ClearFocus)))))

(event EventBeginPlay
  ;[1 1 1] Setup and Store Blackboard in Variable
  (bind _blackboardcomponent (Class|AIController|UseBlackboard "/Game/Dynamic/NPC/AI/PatrolData.PatrolData"))
  (AI|RunBehaviorTree "/Game/Dynamic/NPC/AI/GuardBehavior.GuardBehavior")
  (Variables|Default|SetBlackBoardComp _blackboardcomponent))

(event EventTick
  (params (DeltaSeconds :type Float%20%28single-precision%29))
  (bind _returnvalue (Class|AIController|GetFocusActor))
  (bind _returnvalue_2 (Utilities|IsValid _returnvalue))
  ;[1 1 1] Focus on Player
  (Utilities|FlowControl|Sequence
    (:then_1
      (bind _asue_4asp_character (Utilities|Casting|CastToUe4ASP_Character (Pawn|GetControlledPawn)))
      (Variables|/Game/Dynamic/NPC/Behavior/Ue4ASP_Character.Ue4ASP_Character_C|SetAiming _asue_4asp_character _returnvalue_2)
      (Variables|/Game/Dynamic/NPC/Behavior/Ue4ASP_Character.Ue4ASP_Character_C|SetShooting _asue_4asp_character _returnvalue_2))))

(fn ConstructionScript)

(fn PrintDebugString
  (params (Stimulus :type AI%20Stimulus%20Structure%20%28by%20ref%29) (Object :type Object%20Object%20Reference))
  (bind _returnvalue (Class|AIPerceptionSystem|GetSenseClassforStimulus Stimulus))
  (Development|PrintString (Utilities|String|ToString(Text) (Utilities|Text|FormatText "{Guard} {PerceptionClass} {Actor}" (Utilities|Text|ToText(String) (Utilities|GetObjectName (Pawn|GetControlledPawn))) (Utilities|Text|ToText(String) (Utilities|GetClassDisplayName _returnvalue)) (Utilities|Text|ToText(String) (Utilities|GetObjectName Object))))))